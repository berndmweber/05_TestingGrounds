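; AI controller for guard NPCs that runs a behavior tree and tracks sensed targets.
; On BeginPlay it initializes the PatrolData blackboard and starts the GuardBehavior tree.
; AI Perception updates write sensed actors lacking the "Enemy" tag to the EnemyKey blackboard entry.
; A failed sense of any such actor clears that key, regardless of which actor is stored.
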(event `self.ReceiveBeginPlay`
  ;[1 1 1] Patrol Configuration
  (bind _blackboardcomponent (`self.UseBlackboard` "/Game/Dynamic/NPC/Blueprints/AI/PatrolData.PatrolData"))
  (set `self.BlackboardComponent` _blackboardcomponent)
  (`self.RunBehaviorTree` "/Game/Dynamic/NPC/Blueprints/AI/GuardBehavior.GuardBehavior"))

(event `self.AIPerception.OnTargetPerceptionUpdated`
  (params (Actor :type "Actor Object Reference") (Stimulus :type "AIStimulus Structure"))
  (bind _blackboardcomponent (`self.BlackboardComponent`))
  (bind _enemykey (`self.EnemyKey`))
  ;[1 1 1] Report sensing event
  (if (`self.ActorHasTag` Actor "Enemy")
    _
    (elif (`.bSuccessfullySensed` (break `AIStimulus` Stimulus))
      (`BlackboardComponent.SetValueAsObject` _blackboardcomponent _enemykey Actor)
      (else
        (`BlackboardComponent.ClearValue` _blackboardcomponent _enemykey)))))

(fn `UserConstructionScript`)